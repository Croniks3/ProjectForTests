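; Spline actor that slides a deforming mesh segment of fixed Length along its spline at runtime.
; BeginPlay creates the SplineMesh component and plays a Timeline at SpeedMove rate, whose Rail track maps to distance along the spline.
; Each update sets the segment's ends from world-space spline samples, clamping tangents to Length so the mesh follows curves.
; Updates are skipped once the segment's front reaches the spline end.
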(event `self.ReceiveBeginPlay`
  (bind _length (`self.length`))
  (bind _spline (`self.Spline`))
  (bind _length_2 (`self.length`))
  (bind _returnvalue (`SplineComponent.GetSplineLength` (`self.Spline`)))
  (`TimelineComponent.SetPlayRate` (`self.Timeline`) (`self.speedMove`))
  ;[1 1 1] Меш заменять тут
  (bind _returnvalue_2 (`AddComponent|NODE_AddSplineMeshComponent-0`))
  (bind _output_get (set `self.SplineMesh` _returnvalue_2))
  (`SplineMeshComponent.SetForwardAxis` _returnvalue_2 "X" true)
  (bind (_direction _rail) (`Timeline|Timeline`)
    (:`Update`
      (bind _returnvalue_3 (* _rail _returnvalue))
      (if (not (>= _returnvalue_3 (- _returnvalue _length)))
        (bind _returnvalue_4 (+ _returnvalue_3 _length))
        (`SplineMeshComponent.SetStartAndEnd` _output_get (`SplineComponent.GetLocationAtDistanceAlongSpline` _spline _returnvalue_3 "World") (`KismetMathLibrary.Vector_ClampSizeMax` (`SplineComponent.GetTangentAtDistanceAlongSpline` _spline _returnvalue_3 "World") _length_2) (`SplineComponent.GetLocationAtDistanceAlongSpline` _spline _returnvalue_4 "World") (`KismetMathLibrary.Vector_ClampSizeMax` (`SplineComponent.GetTangentAtDistanceAlongSpline` _spline _returnvalue_4 "World") _length_2) true)))))

(fn `UserConstructionScript`)