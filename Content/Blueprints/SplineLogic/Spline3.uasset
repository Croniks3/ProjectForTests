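; Construction script that populates a spline with repeated spline mesh components, spaced by mesh length plus a spacing value.
; Mesh length comes from the bounding box along the chosen forward axis.
; Each component sits at its distance along the spline, unrotated, without start/end points or tangents set, so nothing bends to the curve.
; The loop count adds section length to spline length instead of dividing, so it far exceeds the sections that fit.
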(fn `UserConstructionScript`
  (bind (_min _max) (break `Box` (`StaticMesh.GetBoundingBox` (`self.SplineMesh`))))
  (bind (_returnvalue_x _returnvalue_y _returnvalue_z) (`KismetMathLibrary.BreakVector` (- _max _min)))
  (if (`|EnumEquality` (`self.In Forward Axis`) "X")
    (set `self.MeshLength` _returnvalue_x)
    (elif (`|EnumEquality` (`self.In Forward Axis`) "Y")
      (set `self.MeshLength` _returnvalue_y)
      (else
        (set `self.MeshLength` _returnvalue_z))))
  (set `self.SectionLength` (+ (`self.MeshLength`) (`self.SpacingLength`)))
  (for _index (range (+ (`KismetMathLibrary.FTrunc` (+ (`SplineComponent.GetSplineLength` (`self.Spline`)) (`self.SectionLength`))) 1))
    (set `self.Index` _index)
    (bind _returnvalue (`AddComponent|NODE_AddSplineMeshComponent-2` :`RelativeTransform` (`KismetMathLibrary.MakeTransform` (`SplineComponent.GetLocationAtDistanceAlongSpline` (`self.Spline`) (* (`self.Index`) (`self.SectionLength`)) "Local"))))
    (`StaticMeshComponent.SetStaticMesh` _returnvalue (`self.SplineMesh`))
    (`SplineMeshComponent.SetForwardAxis` _returnvalue (`self.In Forward Axis`) true)))