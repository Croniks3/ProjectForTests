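; Spline actor that slides a single deforming mesh along its spline path when LaunchSplineMeshMoving is called.
; BeginPlay creates the spline mesh with Y as forward axis, sets the timeline rate from SpeedMove, and caches spline length and the mesh's X-bounds length.
; After a short delay, the timeline re-fits the mesh each update to a mesh-length segment with clamped tangents, stopping when it reaches the spline's end.
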(event `self.ReceiveBeginPlay`
  (`TimelineComponent.SetPlayRate` (`self.SplineTimeline`) (`self.SpeedMove`))
  (bind _returnvalue (`AddComponent|NODE_AddSplineMeshComponent-1`))
  (bind _output_get (set `self.SplineMesh` _returnvalue))
  (`SplineMeshComponent.SetForwardAxis` _output_get "Y" true)
  (`KismetSystemLibrary.Delay` 0.4)
  (`self.Save Dimensions`)
  (`SplineMeshComponent.SetStartAndEnd` (`self.SplineMesh`) (0.0 0.0 0.0) (0.0 0.0 0.0) (0.0 0.0 0.0) (0.0 0.0 0.0) true))

(event `LaunchSplineMeshMoving`
  (`SplineMeshComponent.SetStartAndEnd` (`self.SplineMesh`) (0.0 0.0 0.0) (0.0 0.0 0.0) (0.0 0.0 0.0) (0.0 0.0 0.0) true)
  (`KismetSystemLibrary.Delay` 0.4)
  (bind (_direction _percent) (`Timeline|SplineTimeline` :!via `PlayFromStart`)
    (:`Update`
      (if (>= (+ (* (`self.SplineLength`) _percent) (`self.SplineMeshLengthByX`)) (`self.SplineLength`))
        (`TimelineComponent.Stop` (`self.SplineTimeline`))
        (else
          (bind _returnvalue (* (`self.SplineLength`) _percent))
          (bind _returnvalue_2 (`KismetMathLibrary.FClamp` (+ _returnvalue (`self.SplineMeshLengthByX`)) (`self.SplineMeshLengthByX`) (`self.SplineLength`)))
          (`SplineMeshComponent.SetStartAndEnd` (`self.SplineMesh`) (`SplineComponent.GetLocationAtDistanceAlongSpline` (`self.Spline`) _returnvalue "Local") (`KismetMathLibrary.ClampVectorSize` (`SplineComponent.GetTangentAtDistanceAlongSpline` (`self.Spline`) _returnvalue "Local") 0.0 (`self.SplineMeshLengthByX`)) (`SplineComponent.GetLocationAtDistanceAlongSpline` (`self.Spline`) _returnvalue_2 "Local") (`KismetMathLibrary.ClampVectorSize` (`SplineComponent.GetTangentAtDistanceAlongSpline` (`self.Spline`) _returnvalue_2 "Local") 0.0 (`self.SplineMeshLengthByX`)) true))))))

(fn `Save Dimensions`
  (bind (_min _max) (`StaticMeshComponent.GetLocalBounds` (`self.SplineMesh`)))
  (set `self.SplineLength` (`SplineComponent.GetSplineLength` (`self.Spline`)))
  (set `self.SplineMeshLengthByX` (- (.x _max) (.x _min))))

(fn `UserConstructionScript`)