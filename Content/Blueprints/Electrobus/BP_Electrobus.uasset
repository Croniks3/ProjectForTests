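; Electric bus actor that, on each LaunchBus call, plays audio and alternates between animated drives along two splines, resetting after the second.
; Timelines, rate-scaled by animation time, move the body by spline distance, optionally scaling it up from an initial to target size on the first leg.
; Wheels spin with distance travelled, while front wheels steer by signed tangent-to-forward angle deltas, gated by an accumulated-angle limit.
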(event `self.ReceiveBeginPlay`
  ;[1 1 1] Init
  (if (`self.SplineVisible`)
    (`KismetSystemLibrary.ExecuteConsoleCommand` "ShowFlag.Splines 1" null)
    (else
      (`KismetSystemLibrary.ExecuteConsoleCommand` "ShowFlag.Splines 0" null)))
  (`self.Set Length and Play Rate` (`self.Spline_1`) (`self.SplineLength_1`) (`self.Timeline_1`) (`self.AnimationTime_1`))
  (`self.Set Length and Play Rate` (`self.Spline_2`) (`self.SplineLength_2`) (`self.Timeline_2`) (`self.AnimationTime_2`))
  (set `self.WheelsArray` (`|MakeArray` (`self.FrontLeftWheel`) (`self.FrontRightWheel`) (`self.BackLeftWheel`) (`self.BackRightWheel`)))
  (`self.SetLocationAndRotationBySplineDistance` (`self.Body`) (`self.Spline_1`))
  (if (not (<= (`self.ScaleTimeDuration`) 0.0))
    (`SceneComponent.SetRelativeScale3D` (`self.Body`) (`self.InitScale`))))

(event `LaunchBus`
  ;[1 1 1] Launch
  (`AudioComponent.Play` (`self.Audio`) 0.0)
  (`/Engine/EditorBlueprintResources/StandardMacros.FlipFlop`
    (:`A`
      (`TimelineComponent.Stop` (`self.Timeline_2`))
      (`self.ResetBus`)
      (set `self.CurrentSplineLength` (`self.SplineLength_1`))
      (set `self.CurrentSpline` (`self.Spline_1`))
      (bind (_direction _percent) (`Timeline|Timeline_1` :!via `PlayFromStart`)
        (:`Update`
          (set `self.Percent` _percent)
          (`|ExecutionSequence` :!label _label
            (:`then_0`
              ;[1 1 1] BusBodyMoving
              (bind _resultsteeringangle (`self.CalculateSteeringAngle` (`self.CurrentSpline`) (`self.CurrentSplineLength`)))
              (set `self.CurrentSteeringAngle` _resultsteeringangle)
              (`self.SetLocationAndRotationBySplineDistance` (`self.Body`) (`self.CurrentSpline`) (* (`self.CurrentSplineLength`) (`self.Percent`))))
            (:`then_1`
              ;[1 1 1] WheelsRotationAndTurning
              (bind _wheelrotation (`self.CaclulateWheelRotation` (`self.CurrentSplineLength`)))
              (set `self.CurrentWheelRotation` _wheelrotation)
              (bind _output_get (set `self.DeltaAngle` (* (* (- (`self.CurrentSteeringAngle`) (`self.PreviousSteeringAngle`)) 100.0) (`self.SteeringFactor`))))
              (set `self.AccumulatedAngle` (+ _output_get (`self.AccumulatedAngle`)))
              (for (_array_element _array_index) (`self.WheelsArray`)
                ;;[1 1 1] FourWheelsRotation
                (`SceneComponent.K2_AddLocalRotation` _array_element (`KismetMathLibrary.MakeRotator` 0.0 (- (`self.CurrentWheelRotation`) (`self.PreviousWheelRotation`))) false false)
                ;;[1 1 1] FirstTwoWheelsTurning
                (if (< _array_index 2)
                  (bind _inrangle (`self.CheckAngleInRangle`))
                  (if _inrangle
                    (`SceneComponent.K2_AddWorldRotation` _array_element (`KismetMathLibrary.MakeRotator` 0.0 0.0 (`self.DeltaAngle`)) false false))))
              (set `self.PreviousWheelRotation` (`self.CurrentWheelRotation`))
              (set `self.PreviousSteeringAngle` (`self.CurrentSteeringAngle`)))
            (:`then_2`
              ;[1 1 1] BusBodyScaling
              (if (and (> (`self.ScaleTimeDuration`) 0.0) (!= (`self.CurrentSpline`) (`self.Spline_2`)))
                (`SceneComponent.SetRelativeScale3D` (`self.Body`) (`KismetMathLibrary.VLerp` (`self.InitScale`) (`self.TargetScale`) (`KismetMathLibrary.FClamp` (/ (`self.Percent`) (`self.ScaleTimeDuration`)))))))))))
    (:`B`
      (`TimelineComponent.Stop` (`self.Timeline_1`))
      (set `self.CurrentSplineLength` (`self.SplineLength_2`))
      (set `self.CurrentSpline` (`self.Spline_2`))
      (bind (_direction_2 _percent_2) (`Timeline|Timeline_2` :!via `PlayFromStart`)
        (:`Update`
          (set `self.Percent` _percent_2)
          (goto _label))
        (:`Finished`
          (`self.ResetBus`))))))

(fn `CaclulateWheelRotation`
  (params (SplineLength :type "Float (double-precision) (by ref)"))
  (returns (WheelRotation :type "Float (double-precision)"))
  (return (* (* (/ (* (`local.SplineLength`) (`self.Percent`)) (`KismetMathLibrary.MultiplyByPi` 100.0)) 360.0) -1.0)))

(fn `CalculateSteeringAngle`
  (params (Spline :type "SplineComponent Object Reference (by ref)") (SplineLength :type "Float (double-precision) (by ref)"))
  (returns (ResultSteeringAngle :type "Float (double-precision)"))
  (locals (SteeringAngle :type "Float (double-precision)"))
  (bind _returnvalue (`KismetMathLibrary.Normal` (`SceneComponent.GetForwardVector` (`self.Body`))))
  (bind _returnvalue_2 (`KismetMathLibrary.Normal` (`SplineComponent.GetTangentAtDistanceAlongSpline` (`local.Spline`) (* (`local.SplineLength`) (`self.Percent`)) "World")))
  (bind _returnvalue_3 (`KismetMathLibrary.DegAcos` (`KismetMathLibrary.Dot_VectorVector` _returnvalue _returnvalue_2)))
  (if (>= (`.Z` (`KismetMathLibrary.BreakVector3f` (`KismetMathLibrary.Cross_VectorVector` _returnvalue _returnvalue_2))) 0.0)
    (set `local.SteeringAngle` _returnvalue_3)
    (else
      (set `local.SteeringAngle` (* _returnvalue_3 -1.0))))
  (return (`local.SteeringAngle`)))

(fn `CheckAngleInRangle`
  (returns (InRangle :type Boolean))
  (return (and (<= (`self.AccumulatedAngle`) (`self.MaxSteeringAngle`)) (>= (`self.AccumulatedAngle`) (* (`self.MaxSteeringAngle`) -1.0)))))

(fn `ResetBus`
  (set `self.Percent` 0.0)
  (set `self.CurrentSteeringAngle` 0.0)
  (set `self.PreviousSteeringAngle` 0.0)
  (set `self.CurrentWheelRotation` 0.0)
  (set `self.PreviousWheelRotation` 0.0)
  (set `self.AccumulatedAngle` 0.0)
  (set `self.DeltaAngle` 0.0)
  (set `self.CurrentSplineLength` 0.0)
  (set `self.CurrentSpline` null)
  (`self.SetLocationAndRotationBySplineDistance` (`self.Body`) (`self.Spline_1`))
  (for _index (range 2)
    (`SceneComponent.K2_SetRelativeRotation` :`self` (select `int` _index :`0` (`self.FrontLeftWheel`) :`1` (`self.FrontRightWheel`))))
  (if (not (<= (`self.ScaleTimeDuration`) 0.0))
    (`SceneComponent.SetRelativeScale3D` (`self.Body`) (`self.InitScale`))))

(fn `Set Length and Play Rate`
  (params (Spline :type "SplineComponent Object Reference (by ref)") (SplineLength :type "Float (double-precision) (by ref)") (Timeline :type "TimelineComponent Object Reference (by ref)") (AnimationTime :type "Float (double-precision) (by ref)"))
  (bind _timeline (`local.Timeline`))
  (`|VariableSetRef` (`local.SplineLength`) (`SplineComponent.GetSplineLength` (`local.Spline`)))
  (if (<= (`local.AnimationTime`) 0.0)
    (`TimelineComponent.SetPlayRate` _timeline 0.0)
    (else
      (`TimelineComponent.SetPlayRate` _timeline (/ 1.0 (`local.AnimationTime`))))))

(fn `SetLocationAndRotationBySplineDistance`
  (params (StaticMesh :type "StaticMeshComponent Object Reference (by ref)") (Spline :type "SplineComponent Object Reference (by ref)") (Distance :type "Float (double-precision)"))
  (`SceneComponent.K2_SetWorldLocationAndRotation` StaticMesh (`SplineComponent.GetLocationAtDistanceAlongSpline` (`local.Spline`) (`local.Distance`) "World") (`SplineComponent.GetRotationAtDistanceAlongSpline` (`local.Spline`) (`local.Distance`) "World") false false))

(fn `UserConstructionScript`
  (`self.SetLocationAndRotationBySplineDistance` (`self.Body`) (`self.Spline_1`))
  (if (not (<= (`self.ScaleTimeDuration`) 0.0))
    (`SceneComponent.SetRelativeScale3D` (`self.Body`) (`self.TargetScale`))))